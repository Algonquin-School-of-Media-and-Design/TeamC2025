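; BP_TempWall is a temporary wall that displays a spawn point's wave progress and disappears once all its waves are finished.
; Every Tick, the authority builds a "Waves: current/total" string from the referenced spawn point and destroys the wall when that spawn point reports completion.
; Otherwise the WaveCount text is updated from the stored string, which remote instances display without recomputing it.
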(event EventBeginPlay)

(event Collision|EventActorBeginOverlap
  (params (OtherActor :type Actor%20Object%20Reference)))

(event EventTick
  (params (DeltaSeconds :type Float%20%28single-precision%29))
  (bind _spawnpointreff (Variables|Default|GetSpawnPointReff))
  (Networking|SwitchHasAuthority
    (:Authority
      (Variables|Default|Setstringrep (Utilities|String|ToString(Text) (Utilities|Text|ToText(String) (Utilities|String|Append (Utilities|String|Append (Utilities|String|Append "Waves: " (Utilities|String|ToString(Integer) (Variables|/Script/RelicRunners.SpawnPoint|Getm_CurrentWaves _spawnpointreff))) "/") (Utilities|String|ToString(Integer) (Variables|/Script/RelicRunners.SpawnPoint|Getm_numOfWaves _spawnpointreff))))))
      (bind _returnvalue (Class|SpawnPoint|FinishedAllWaves (Variables|Default|GetSpawnPointReff)))
      (if _returnvalue
        (Actor|DestroyActor)
        (else
          (Rendering|Components|TextRender|SetText (Variables|Default|GetWaveCount) (Utilities|Text|ToText(String) (Variables|Default|Getstringrep)) :!label _label))))
    (:Remote
      (goto _label))))

(fn ConstructionScript)