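; Anim notify state that opens a hit window for an enemy's basic attack during the animation.
; On begin, it binds an event to the owner character's AttackOverlapCollider begin-overlap and enables query-only collision.
; On end, it unbinds all begin-overlap events from that collider and disables its collision, so overlaps only register within the notify's span.
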(fn ReceivedNotifyBegin
  (params (MeshComp :type Skeletal%20Mesh%20Component%20Object%20Reference) (Animation :type Anim%20Sequence%20Base%20Object%20Reference) (TotalDuration :type Float%20%28single-precision%29) (EventReference :type Anim%20Notify%20Event%20Reference%20Structure%20%28by%20ref%29))
  (bind _ownercharacter (Variables|Default|GetOwnerCharacter))
  (bind _attackoverlapcollider (Variables|/Script/RelicRunners.TormentedSoulCharacter|GetAttackOverlapCollider _ownercharacter))
  (|CallParentFunction MeshComp Animation TotalDuration EventReference)
  (Collision|BindEventtoOnComponentBeginOverlap _attackoverlapcollider (EventDispatchers|CreateEvent _ownercharacter :!event BasicAttack))
  (Collision|SetCollisionEnabled _attackoverlapcollider "QueryOnly")
  (return false))

(fn ReceivedNotifyEnd
  (params (MeshComp :type Skeletal%20Mesh%20Component%20Object%20Reference) (Animation :type Anim%20Sequence%20Base%20Object%20Reference) (EventReference :type Anim%20Notify%20Event%20Reference%20Structure%20%28by%20ref%29))
  (bind _ownercharacter (Variables|Default|GetOwnerCharacter))
  (bind _attackoverlapcollider (Variables|/Script/RelicRunners.TormentedSoulCharacter|GetAttackOverlapCollider _ownercharacter))
  (|CallParentFunction MeshComp Animation EventReference)
  (EventDispatchers|UnbindallEventsfromOnComponentBeginOverlap _attackoverlapcollider)
  (Collision|SetCollisionEnabled _attackoverlapcollider "NoCollision")
  (return false))