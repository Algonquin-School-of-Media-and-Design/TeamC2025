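; AI controller for the Tormented Soul enemy that runs its behavior tree and tracks players by sight.
; On possess it starts the tree, then a tick later seeds the blackboard with itself and its controlled character.
; Sight perception updates set TargetActor when a RelicRunnersCharacter is seen, or clear it and store LastSeenLocation when sight is lost.
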(event OnTargetPerceptionUpdated(AIPerceptionComp)
  (params (Actor :type Actor%20Object%20Reference) (Stimulus :type AI%20Stimulus%20Structure))
  (CallFunction|HandleSightSense Actor Stimulus))

(event EventBeginPlay)

(event EventTick
  (params (DeltaSeconds :type Float%20%28single-precision%29)))

(event EventPossess
  (params (PossessedPawn :type Pawn%20Object%20Reference))
  (AI|RunBehaviorTree (Variables|Default|GetStartingBehaviorTree))
  (Utilities|FlowControl|DelayUntilNextTick)
  (CallFunction|SetUpBlackBoard))

(fn ConstructionScript)

(fn HandleSightSense
  (params (InputActor :type Actor%20Object%20Reference) (Stimulus :type AI%20Stimulus%20Structure))
  (bind (_age _expirationage _strength _stimuluslocation _receiverlocation _tag _bsuccessfullysensed) (Utilities|Struct|BreakAIStimulus Stimulus))
  (bind _returnvalue (Class|AIPerceptionSystem|GetSenseClassforStimulus Stimulus))
  (if (== _returnvalue "/Script/AIModule.AISense_Sight")
    (bind _outactors (Actor|GetAllActorsOfClass "/Script/RelicRunners.RelicRunnersCharacter"))
    (for _array_element _outactors
      (if (== InputActor _array_element)
        (AI|Components|Blackboard|SetValueasObject (Variables|Default|GetBlackboard) (Utilities|Name|MakeLiteralName "TargetActor") (Utilities|SelectObject _array_element 0 _bsuccessfullysensed))
        (if _bsuccessfullysensed
          (return)
          (else
            (AI|Components|Blackboard|SetValueasVector (Variables|Default|GetBlackboard) (Utilities|Name|MakeLiteralName "LastSeenLocation") _stimuluslocation)
            (return)))))
    (return)
    (else
      (return))))

(fn SetUpBlackBoard
  (bind _astormented_soul_character (Utilities|Casting|CastToTormentedSoulCharacter (Pawn|GetControlledPawn)))
  (AI|Components|Blackboard|SetValueasObject (Variables|Default|GetBlackboard) (Utilities|Name|MakeLiteralName "TormentedSoulCharacter") _astormented_soul_character)
  (AI|Components|Blackboard|SetValueasObject (Variables|Default|GetBlackboard) (Utilities|Name|MakeLiteralName "TormentedSoulAIController") self)
  (return))